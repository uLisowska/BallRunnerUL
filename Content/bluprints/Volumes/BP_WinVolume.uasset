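; BP_WinVolume is a level exit volume that advances the game when the player overlaps it with all crystals collected.
; On overlap it checks whether any Crystal actors remain in the world via GetAllActorsOfClass.
; If none remain, it finds the current level's name in the LevelName array and opens the next entry.
; On the final level in that array, completion does nothing further.
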(event `self.ReceiveActorBeginOverlap`
  (params (OtherActor :type "Actor Object Reference"))
  (`/Game/bluprints/Libraries/NewMacroLibrary.Is Player` OtherActor
    (:`true`
      (if (not (`self.any crystal remaining`))
        (`self.Comlete level`)))))

(fn `any crystal remaining`
  (returns (ReturnValue :type Boolean))
  (bind _outactors (`GameplayStatics.GetAllActorsOfClass` "/Game/bluprints/pawns/crysdtalas/crystal.crystal_C"))
  (return (> (`KismetArrayLibrary.Array_Length` _outactors) 0)))

(fn `Comlete level`
  (if (not (`self.Is Final Level`))
    (`self.Load Next Level`)))

(fn `Get Current level index`
  (returns (`Return Value` :type Integer))
  (bind _returnvalue (`GameplayStatics.GetCurrentLevelName` true))
  (return (`KismetArrayLibrary.Array_Find` (`self.Level Name`) (`KismetStringLibrary.Conv_StringToName` _returnvalue))))

(fn `Get nexrt level name`
  (returns (`Retur Value` :type Name))
  (return (`|GetArrayItem` (`self.Level Name`) (+ (`self.Get Current level index`) 1))))

(fn `Is Final Level`
  (returns (`Return Value` :type Boolean))
  (return (== (`KismetArrayLibrary.Array_LastIndex` (`self.Level Name`)) (`self.Get Current level index`))))

(fn `Load Next Level`
  (`GameplayStatics.OpenLevel` (`self.Get nexrt level name`)))

(fn `UserConstructionScript`)